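; BP_TowerBoundary is a world actor that builds a U-shaped tower boundary from mesh instances: a base row and two tall side walls.
; The construction script adds scaled InstancedStaticMesh instances in local space, mirroring the base along X and stacking the walls up Z.
; The wall loop is nested inside the base loop, so every pass stacks duplicate wall instances at identical positions.
; The event graph has no active logic.
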(fn `UserConstructionScript`
  (for _index (range 14)
    (`InstancedStaticMeshComponent.AddInstance` (`self.InstancedStaticMesh`) (`KismetMathLibrary.MakeTransform` (`KismetMathLibrary.MakeVector` (`KismetMathLibrary.Conv_IntToDouble` (* _index -100))) (struct) (1.0 4.0 2.0)) false)
    (`InstancedStaticMeshComponent.AddInstance` (`self.InstancedStaticMesh`) (`KismetMathLibrary.MakeTransform` (`KismetMathLibrary.MakeVector` (`KismetMathLibrary.Conv_IntToDouble` (* _index 100))) (struct) (1.0 4.0 2.0)) false)
    (for _index_2 (range 51)
      (`InstancedStaticMeshComponent.AddInstance` (`self.InstancedStaticMesh`) (`KismetMathLibrary.MakeTransform` (`KismetMathLibrary.MakeVector` 1300.0 0.0 (`KismetMathLibrary.Conv_IntToDouble` (* _index_2 100))) (struct) (2.0 4.0 1.0)) false)
      (`InstancedStaticMeshComponent.AddInstance` (`self.InstancedStaticMesh`) (`KismetMathLibrary.MakeTransform` (`KismetMathLibrary.MakeVector` -1300.0 0.0 (`KismetMathLibrary.Conv_IntToDouble` (* _index_2 100))) (struct) (2.0 4.0 1.0)) false))))