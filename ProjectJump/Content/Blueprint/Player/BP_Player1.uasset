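; 2D side-view player character with Enhanced Input walking, a hold-to-charge jump and fall damage.
; Hold time sets a clamped launch strength, shown as text while charging; charging and landing lock walking, with no unlock in this Blueprint.
; Airborne/Landed animation node jumps follow movement events, and Tick flips facing through controller yaw.
; BeginFall/EndFall measure drop height for tiered self-damage, handled by AnyDamage as a red flash or death.
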(event `self.ReceiveTick`
  (params (DeltaSeconds :type "Float (single-precision)"))
  (bind _returnvalue (`self.GetController`))
  (bind _returnvalue_2 (`self.GetController`))
  (bind _velocity_x (`KismetMathLibrary.BreakVector` (`MovementComponent.Velocity` (`self.GetMovementComponent`))))
  ;[1 1 1] Sprite Flipping
  (`parent.ReceiveTick` 0.0)
  (`/Engine/EditorBlueprintResources/StandardMacros.CompareFloat` _velocity_x
    (:`>`
      (`/Engine/EditorBlueprintResources/StandardMacros.IsValid` _returnvalue_2
        (:`Is Valid`
          (`Controller.SetControlRotation` _returnvalue_2 (`KismetMathLibrary.MakeRotator` 0.0)))))
    (:`<`
      (`/Engine/EditorBlueprintResources/StandardMacros.IsValid` _returnvalue
        (:`Is Valid`
          (`Controller.SetControlRotation` _returnvalue (`KismetMathLibrary.MakeRotator` 0.0 0.0 180.0)))))))

(event `self.ReceiveBeginPlay`
  ;[1 1 1] Begin Play / Setting Up Mapping
  (bind _asplayer_controller (cast `PlayerController` (`self.GetController`)))
  (bind _returnvalue (pcsubsystem `EnhancedInputLocalPlayerSubsystem` _asplayer_controller))
  (`/Engine/EditorBlueprintResources/StandardMacros.IsValid` _returnvalue
    (:`Is Valid`
      (`EnhancedInputSubsystemInterface.AddMappingContext` _returnvalue "/Game/Blueprint/Player/Player_InputMap.Player_InputMap" 0 (struct)))))

(event `self.OnWalkingOffLedge`
  (params (PreviousFloorImpactNormal :type "Vector Structure (by ref)") (PreviousFloorContactNormal :type "Vector Structure (by ref)") (PreviousLocation :type "Vector Structure (by ref)") (TimeDelta :type "Float (single-precision)"))
  ;[1 1 1] Anim Events
  (`PaperZDAnimInstance.JumpToNode` (`PaperZDAnimationComponent.AnimInstance` (`self.AnimationComponent`)) "Airborne" "None"))

(event `EnhancedInput|/Game/Blueprint/Player/InputActions/IA_Player_Jump`
  (params (ActionValue :type Boolean) (ElapsedSeconds :type "Float (double-precision)") (TriggeredSeconds :type "Float (double-precision)") (InputAction :type "InputAction Object Reference" :default "/Game/Blueprint/Player/InputActions/IA_Player_Jump.IA_Player_Jump"))
  (bind _charactermovement (`self.CharacterMovement`))
  ;[1 1 1] Jump Event
  (:`Started`
    (`PaperZDAnimInstance.JumpToNode` (`PaperZDAnimationComponent.AnimInstance` (`self.AnimationComponent`)) "Airborne" "None"))
  (:`Ongoing`
    (set `self.IsMovementLocked` true)
    (if (not (`NavMovementComponent.IsFalling` (`self.CharacterMovement`)))
      (`TextRenderComponent.K2_SetText` (`self.TheTextBox`) (`KismetTextLibrary.Conv_DoubleToText` (`KismetMathLibrary.Conv_IntToDouble` (`KismetMathLibrary.Clamp` (`KismetMathLibrary.FTrunc` (* ElapsedSeconds (`self.JumpStrength`))) 50 1000)) "HalfToEven"))))
  (:`Completed`
    (set `CharacterMovementComponent.AirControl` (`self.PlayerAirCtrl`) _charactermovement)
    (if (not (`NavMovementComponent.IsFalling` _charactermovement))
      (`self.LaunchCharacter` (`KismetMathLibrary.MakeVector` 0.0 0.0 (`KismetMathLibrary.Conv_IntToDouble` (`KismetMathLibrary.Clamp` (`KismetMathLibrary.FTrunc` (* ElapsedSeconds (`self.JumpStrength`))) 50 1000)))))))

(event `self.OnLanded`
  (params (Hit :type "HitResult Structure (by ref)"))
  ;[1 1 1] Anim Events
  (`PaperZDAnimInstance.JumpToNode` (`PaperZDAnimationComponent.AnimInstance` (`self.AnimationComponent`)) "Landed" "None")
  (`MovementComponent.StopMovementImmediately` (`self.CharacterMovement`))
  (set `self.IsMovementLocked` true))

(event `self.OnLaunched`
  (params (LaunchVelocity :type "Vector Structure") (bXYOverride :type Boolean) (bZOverride :type Boolean))
  ;[1 1 1] Anim Events
  (`PaperZDAnimInstance.JumpToNode` (`PaperZDAnimationComponent.AnimInstance` (`self.AnimationComponent`)) "Airborne" "None"))

(event `EnhancedInput|/Game/Blueprint/Player/InputActions/IA_Player_Walk`
  (params (ActionValue :type "Vector2D Structure") (ElapsedSeconds :type "Float (double-precision)") (TriggeredSeconds :type "Float (double-precision)") (InputAction :type "InputAction Object Reference" :default "/Game/Blueprint/Player/InputActions/IA_Player_Walk.IA_Player_Walk"))
  ;[1 1 1] Walk Event
  (:`Triggered`
    (if (not (`self.IsMovementLocked`))
      (`self.AddMovementInput` (`KismetMathLibrary.MakeVector` ActionValue_X)))))

(event `self.ReceiveAnyDamage`
  (params (Damage :type "Float (single-precision)") (DamageType :type "DamageType Object Reference") (InstigatedBy :type "Controller Object Reference") (DamageCauser :type "Actor Object Reference"))
  ;[1 1 1] Take Damage Event
  (set `self.CurrentHealth` (`KismetMathLibrary.FClamp` (- (`self.CurrentHealth`) Damage) 0.0 (`self.MaxHealth`)))
  (if (<= (`self.CurrentHealth`) 0.0)
    (set `self.IsDead` true)
    (`PaperFlipbookComponent.SetSpriteColor` :`self` (`self.Sprite`))
    (`self.DisableInput` null)
    (else
      (`PaperFlipbookComponent.SetSpriteColor` (`self.Sprite`) (struct :`R` 1.0 :`B` 0.051767 :`A` 1.0))
      (`KismetSystemLibrary.Delay` 0.2)
      (`PaperFlipbookComponent.SetSpriteColor` (`self.Sprite`) (struct :`R` 1.0 :`G` 1.0 :`B` 1.0 :`A` 1.0)))))

(event `Begin Fall`
  ;[1 1 1] Fall Damage Event
  (set `self.FallPosition` (`self.K2_GetActorLocation`)))

(event `End Fall`
  (bind (_returnvalue_x _returnvalue_y _returnvalue_z) (`KismetMathLibrary.BreakVector` (`self.K2_GetActorLocation`)))
  (bind (_fallposition_x _fallposition_y _fallposition_z) (`KismetMathLibrary.BreakVector` (`self.FallPosition`)))
  (bind _returnvalue (- _fallposition_z _returnvalue_z))
  ;[1 1 1] Fall Damage Event
  (if (>= _returnvalue (`self.FallDamageCutoff`))
    (`self.Calculate Fall Damage` _returnvalue))
  (set `self.FallPosition` (`self.K2_GetActorLocation`)))

(event `Calculate Fall Damage`
  (params (`Fall Height` :type "Float (double-precision)"))
  ;[1 1 1] Calculate Fall Damage Amount
  (if (<= `Fall Height` (+ (`self.FallDamageCutoff`) 20.0))
    (set `self.Base Damage` 30.0)
    (elif (<= `Fall Height` (+ (`self.FallDamageCutoff`) 50.0))
      (set `self.Base Damage` 60.0)
      (else
        (set `self.Base Damage` 100.0))))
  (`GameplayStatics.ApplyDamage` self (`self.Base Damage`))
  (set `self.Base Damage` 0.0))

(fn `SpawnDust`
  (bind (_returnvalue_location _returnvalue_rotation) (`KismetMathLibrary.BreakTransform` (`SceneComponent.K2_GetComponentToWorld` (`self.Sprite`))))
  (`|SpawnActorFromClass` "/Game/Blueprint/Player/BP_LandingDust.BP_LandingDust_C" (`KismetMathLibrary.MakeTransform` _returnvalue_location _returnvalue_rotation) "Undefined" "MultiplyWithRoot" null null))

(fn `UserConstructionScript`)