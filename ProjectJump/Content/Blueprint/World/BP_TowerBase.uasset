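; BP_TowerBase is a one-way tower platform that grows the tower upward as the player jumps through it.
; Its construction script lays a row of instanced meshes, whose collision switches off while the player overlaps the Underneath trigger.
; Leaving that trigger restores collision, increments LevelCount and spawns a random platform, boundary and one-way platform at heights scaled by the count.
; The Above trigger toggles input and a gate intended for dropping through.
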(event `self.InstancedStaticMesh.OnComponentBeginOverlap`
  (params (OverlappedComponent :type "PrimitiveComponent Object Reference") (OtherActor :type "Actor Object Reference") (OtherComp :type "PrimitiveComponent Object Reference") (OtherBodyIndex :type Integer) (bFromSweep :type Boolean) (SweepResult :type "HitResult Structure (by ref)")))

(event `self.InstancedStaticMesh.OnComponentHit`
  (params (HitComponent :type "PrimitiveComponent Object Reference") (OtherActor :type "Actor Object Reference") (OtherComp :type "PrimitiveComponent Object Reference") (NormalImpulse :type "Vector Structure") (Hit :type "HitResult Structure (by ref)")))

(event `self.Underneath.OnComponentBeginOverlap`
  (params (OverlappedComponent :type "PrimitiveComponent Object Reference") (OtherActor :type "Actor Object Reference") (OtherComp :type "PrimitiveComponent Object Reference") (OtherBodyIndex :type Integer) (bFromSweep :type Boolean) (SweepResult :type "HitResult Structure (by ref)"))
  ;[1 1 1] Jump up through platform
  (cast `/Game/Blueprint/Player/ConnorsPlayer/Connor_BP_Player` OtherActor)
  (`PrimitiveComponent.SetCollisionEnabled` (`self.InstancedStaticMesh`) "NoCollision"))

(event `self.Underneath.OnComponentEndOverlap`
  (params (OverlappedComponent :type "PrimitiveComponent Object Reference") (OtherActor :type "Actor Object Reference") (OtherComp :type "PrimitiveComponent Object Reference") (OtherBodyIndex :type Integer))
  ;[1 1 1] Jump up through platform
  (cast `/Game/Blueprint/Player/ConnorsPlayer/Connor_BP_Player` OtherActor)
  (`PrimitiveComponent.SetCollisionEnabled` (`self.InstancedStaticMesh`) "QueryAndPhysics")
  (set `self.LevelCount` (+ 1 (`self.LevelCount`)))
  (`|SpawnActorFromClass` "/Game/Blueprint/World/BP_RandomPlatform.BP_RandomPlatform_C" (`KismetMathLibrary.MakeTransform` (`KismetMathLibrary.MakeVector` -1200.0 0.0 (`KismetMathLibrary.Conv_IntToDouble` (* (`self.LevelCount`) 5000)))) "Undefined" "MultiplyWithRoot" null null)
  (`|SpawnActorFromClass` "/Game/Blueprint/World/BP_TowerBoundary.BP_TowerBoundary_C" (`KismetMathLibrary.MakeTransform` (`KismetMathLibrary.MakeVector` 0.0 0.0 (`KismetMathLibrary.Conv_IntToDouble` (* (`self.LevelCount`) 4820)))) "Undefined" "MultiplyWithRoot" null null)
  (`|SpawnActorFromClass` "/Game/Blueprint/World/BP_OneWayPlatform.BP_OneWayPlatform_C" (`KismetMathLibrary.MakeTransform` (`KismetMathLibrary.MakeVector` -1250.0 0.0 (`KismetMathLibrary.Conv_IntToDouble` (* (`self.LevelCount`) 5000)))) "Undefined" "MultiplyWithRoot" null null))

(event `InputAction|Fall through platform`
  (params (Key :type "Key Structure"))
  ;[1 1 1] Fall through platfrom (on pressing s))
)

(event `self.Above.OnComponentBeginOverlap`
  (params (OverlappedComponent :type "PrimitiveComponent Object Reference") (OtherActor :type "Actor Object Reference") (OtherComp :type "PrimitiveComponent Object Reference") (OtherBodyIndex :type Integer) (bFromSweep :type Boolean) (SweepResult :type "HitResult Structure (by ref)"))
  ;[1 1 1] Fall through platfrom (on pressing s))
  (cast `/Game/Blueprint/Player/BP_Player` OtherActor)
  (`self.EnableInput` (`GameplayStatics.GetPlayerController` 0))
  (`/Engine/EditorBlueprintResources/StandardMacros.Gate` true :!via `Open` :!label _label
    (:`Exit`
      (`PrimitiveComponent.SetCollisionEnabled` (`self.InstancedStaticMesh`) "NoCollision"))))

(event `self.Above.OnComponentEndOverlap`
  (params (OverlappedComponent :type "PrimitiveComponent Object Reference") (OtherActor :type "Actor Object Reference") (OtherComp :type "PrimitiveComponent Object Reference") (OtherBodyIndex :type Integer))
  ;[1 1 1] Fall through platfrom (on pressing s))
  (cast `/Game/Blueprint/Player/BP_Player` OtherActor)
  (`self.DisableInput` (`GameplayStatics.GetPlayerController` 0))
  (goto _label :!via `Close`))

(fn `UserConstructionScript`
  (for _index (range 10)
    (`InstancedStaticMeshComponent.AddInstance` (`self.InstancedStaticMesh`) (`KismetMathLibrary.MakeTransform` (`KismetMathLibrary.MakeVector` (`KismetMathLibrary.Conv_IntToDouble` (* _index 256)))) false)))