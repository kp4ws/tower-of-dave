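; Player character Blueprint with a charged jump, where input time sets launch strength.
; BeginPlay adds the Player_InputMap Enhanced Input mapping context to the local player.
; While IA_Player_Jump is ongoing, TheTextBox shows the scaled, clamped elapsed time as a charge value.
; When the action triggers, LaunchCharacter applies that same value as upward velocity, and Started only prints a debug string.
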(event `self.ReceiveBeginPlay`
  (bind _asplayer_controller (cast `PlayerController` (`self.GetController`)))
  (bind _returnvalue (pcsubsystem `EnhancedInputLocalPlayerSubsystem` _asplayer_controller))
  (`/Engine/EditorBlueprintResources/StandardMacros.IsValid` _returnvalue
    (:`Is Valid`
      (`EnhancedInputSubsystemInterface.AddMappingContext` _returnvalue "/Game/Blueprint/Player/Player_InputMap.Player_InputMap" 0 (struct)))))

(event `EnhancedInput|/Game/Blueprint/Player/InputActions/IA_Player_Jump`
  (params (ActionValue :type Boolean) (ElapsedSeconds :type "Float (double-precision)") (TriggeredSeconds :type "Float (double-precision)") (InputAction :type "InputAction Object Reference" :default "/Game/Blueprint/Player/InputActions/IA_Player_Jump.IA_Player_Jump"))
  (:`Triggered`
    (`self.LaunchCharacter` (`KismetMathLibrary.MakeVector` 0.0 0.0 (`KismetMathLibrary.Conv_IntToDouble` (`KismetMathLibrary.Clamp` (`KismetMathLibrary.FTrunc` (* ElapsedSeconds 600.0)) 50 1000)))))
  (:`Started`
    (`KismetSystemLibrary.PrintString` "Start"))
  (:`Ongoing`
    (`TextRenderComponent.K2_SetText` (`self.TheTextBox`) (`KismetTextLibrary.Conv_DoubleToText` (`KismetMathLibrary.Conv_IntToDouble` (`KismetMathLibrary.Clamp` (`KismetMathLibrary.FTrunc` (* ElapsedSeconds 600.0)) 50 1000)) "HalfToEven"))))

(fn `UserConstructionScript`)