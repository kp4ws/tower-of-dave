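; One-way platform actor that scatters randomly placed blocks in vertically spaced rows, which the player can jump up through or drop through.
; The construction script adds instanced static meshes at random slots per row, capped by MaxBlocks.
; An Underneath overlap disables collision while the player is inside.
; An Above overlap enables input and opens a gate for the fall-through action, with collision toggled on the whole instanced component.
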(event `self.Underneath.OnComponentBeginOverlap`
  (params (OverlappedComponent :type "PrimitiveComponent Object Reference") (OtherActor :type "Actor Object Reference") (OtherComp :type "PrimitiveComponent Object Reference") (OtherBodyIndex :type Integer) (bFromSweep :type Boolean) (SweepResult :type "HitResult Structure (by ref)"))
  ;[1 1 1] Jump up through platform
  (cast `/Game/Blueprint/Player/BP_Player` OtherActor)
  (`PrimitiveComponent.SetCollisionEnabled` (`self.InstancedStaticMesh`) "NoCollision"))

(event `self.Underneath.OnComponentEndOverlap`
  (params (OverlappedComponent :type "PrimitiveComponent Object Reference") (OtherActor :type "Actor Object Reference") (OtherComp :type "PrimitiveComponent Object Reference") (OtherBodyIndex :type Integer))
  ;[1 1 1] Jump up through platform
  (cast `/Game/Blueprint/Player/BP_Player` OtherActor)
  (`PrimitiveComponent.SetCollisionEnabled` (`self.InstancedStaticMesh`) "QueryAndPhysics"))

(event `InputAction|Fall through platform`
  (params (Key :type "Key Structure"))
  ;[1 1 1] Fall through platfrom (on pressing s))
  (:`Pressed`
    (`/Engine/EditorBlueprintResources/StandardMacros.Gate` true :!label _label
      (:`Exit`
        (`PrimitiveComponent.SetCollisionEnabled` (`self.InstancedStaticMesh`) "NoCollision")))))

(event `self.Above.OnComponentBeginOverlap`
  (params (OverlappedComponent :type "PrimitiveComponent Object Reference") (OtherActor :type "Actor Object Reference") (OtherComp :type "PrimitiveComponent Object Reference") (OtherBodyIndex :type Integer) (bFromSweep :type Boolean) (SweepResult :type "HitResult Structure (by ref)"))
  ;[1 1 1] Fall through platfrom (on pressing s))
  (cast `/Game/Blueprint/Player/BP_Player` OtherActor)
  (`self.EnableInput` (`GameplayStatics.GetPlayerController` 0))
  (goto _label :!via `Open`))

(event `self.Above.OnComponentEndOverlap`
  (params (OverlappedComponent :type "PrimitiveComponent Object Reference") (OtherActor :type "Actor Object Reference") (OtherComp :type "PrimitiveComponent Object Reference") (OtherBodyIndex :type Integer))
  ;[1 1 1] Fall through platfrom (on pressing s))
  (cast `/Game/Blueprint/Player/BP_Player` OtherActor)
  (`self.DisableInput` (`GameplayStatics.GetPlayerController` 0))
  (goto _label :!via `Close`))

(fn `UserConstructionScript`
  (for _ (range 19)
    (set `self.PlatformSpacing` (+ (`self.PlatformSpacing`) 1250))
    (set `self.BlockCount` 0)
    (for _index (range 9)
      (`/Engine/EditorBlueprintResources/StandardMacros.CompareInt` (`self.BlockCount`) (`self.MaxBlocks`)
        (:`<`
          (`/Engine/EditorBlueprintResources/StandardMacros.CompareInt` (`KismetMathLibrary.RandomInteger` 4) 1
            (:`<`
              (set `self.BlockCount` (+ (`self.BlockCount`) 1))
              (`InstancedStaticMeshComponent.AddInstance` (`self.InstancedStaticMesh`) (`KismetMathLibrary.MakeTransform` (`KismetMathLibrary.MakeVector` (`KismetMathLibrary.Conv_IntToDouble` (* _index 256)) 0.0 (`KismetMathLibrary.Conv_IntToDouble` (`self.PlatformSpacing`))) (struct) (`KismetMathLibrary.MakeVector` (`KismetMathLibrary.Conv_IntToDouble` (+ (`KismetMathLibrary.RandomInteger` 1) 1)) 1.0 1.0)) false))))))))