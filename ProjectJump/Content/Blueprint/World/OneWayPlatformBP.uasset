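; One-way platform actor that the player can jump up through and drop down from on input.
; An Underneath trigger disables the Cube's collision when Player_BP enters and restores it on exit.
; An Above trigger enables the actor's input and opens a gate while the player overlaps it, letting the fall-through action disable collision.
; Only the Underneath exit restores collision, including after a drop.
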(event `self.Underneath.OnComponentBeginOverlap`
  (params (OverlappedComponent :type "PrimitiveComponent Object Reference") (OtherActor :type "Actor Object Reference") (OtherComp :type "PrimitiveComponent Object Reference") (OtherBodyIndex :type Integer) (bFromSweep :type Boolean) (SweepResult :type "HitResult Structure (by ref)"))
  ;[1 1 1] Jump up through platform
  (cast `/Game/Blueprint/Player/Player_BP` OtherActor)
  (`PrimitiveComponent.SetCollisionEnabled` (`self.Cube`) "NoCollision"))

(event `self.Underneath.OnComponentEndOverlap`
  (params (OverlappedComponent :type "PrimitiveComponent Object Reference") (OtherActor :type "Actor Object Reference") (OtherComp :type "PrimitiveComponent Object Reference") (OtherBodyIndex :type Integer))
  ;[1 1 1] Jump up through platform
  (cast `/Game/Blueprint/Player/Player_BP` OtherActor)
  (`PrimitiveComponent.SetCollisionEnabled` (`self.Cube`) "QueryAndPhysics"))

(event `InputAction|Fall through platform`
  (params (Key :type "Key Structure"))
  ;[1 1 1] Fall through platfrom (on pressing s))
  (:`Pressed`
    (`/Engine/EditorBlueprintResources/StandardMacros.Gate` true :!label _label
      (:`Exit`
        (`PrimitiveComponent.SetCollisionEnabled` (`self.Cube`) "NoCollision")))))

(event `self.Above.OnComponentBeginOverlap`
  (params (OverlappedComponent :type "PrimitiveComponent Object Reference") (OtherActor :type "Actor Object Reference") (OtherComp :type "PrimitiveComponent Object Reference") (OtherBodyIndex :type Integer) (bFromSweep :type Boolean) (SweepResult :type "HitResult Structure (by ref)"))
  ;[1 1 1] Fall through platfrom (on pressing s))
  (cast `/Game/Blueprint/Player/Player_BP` OtherActor)
  (`self.EnableInput` (`GameplayStatics.GetPlayerController` 0))
  (goto _label :!via `Open`))

(event `self.Above.OnComponentEndOverlap`
  (params (OverlappedComponent :type "PrimitiveComponent Object Reference") (OtherActor :type "Actor Object Reference") (OtherComp :type "PrimitiveComponent Object Reference") (OtherBodyIndex :type Integer))
  ;[1 1 1] Fall through platfrom (on pressing s))
  (cast `/Game/Blueprint/Player/Player_BP` OtherActor)
  (`self.DisableInput` (`GameplayStatics.GetPlayerController` 0))
  (goto _label :!via `Close`))

(fn `UserConstructionScript`)