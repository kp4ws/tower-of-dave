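; One-way platform built from ten instanced meshes that the player jumps up through, doubling as the trigger for endless tower generation.
; The Underneath overlap toggles collision off and back on.
; Its first exit pays the player and spawns the next LevelCount-based section: random platform, boundary, billboard, shop door and another one-way platform.
; Repeated exits print an anti-cheese warning; the Above fall-through logic is only partly wired.
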(event `self.Underneath.OnComponentBeginOverlap`
  (params (OverlappedComponent :type "PrimitiveComponent Object Reference") (OtherActor :type "Actor Object Reference") (OtherComp :type "PrimitiveComponent Object Reference") (OtherBodyIndex :type Integer) (bFromSweep :type Boolean) (SweepResult :type "HitResult Structure (by ref)"))
  ;[1 1 1] Jump up through platform
  (cast `/Game/Blueprint/Player/ConnorsPlayer/Connor_BP_Player` OtherActor)
  (`PrimitiveComponent.SetCollisionEnabled` (`self.InstancedStaticMesh`) "NoCollision"))

(event `self.Underneath.OnComponentEndOverlap`
  (params (OverlappedComponent :type "PrimitiveComponent Object Reference") (OtherActor :type "Actor Object Reference") (OtherComp :type "PrimitiveComponent Object Reference") (OtherBodyIndex :type Integer))
  (bind _returnvalue (* (`self.LevelCount`) 20))
  ;[1 1 1] Infinite Spawn
  (bind _asconnor_bp_player (cast `/Game/Blueprint/Player/ConnorsPlayer/Connor_BP_Player` OtherActor))
  (`PrimitiveComponent.SetCollisionEnabled` (`self.InstancedStaticMesh`) "QueryAndPhysics")
  (if (`self.SpawnPerformed`)
    (bind _output_get (set `self.PokeCount` (+ (stale _output_get) 1)))
    (`/Engine/EditorBlueprintResources/StandardMacros.CompareInt` (`self.PokeCount`) 5
      (:`>`
        _)
      (:`==`
        _))
    (`KismetSystemLibrary.PrintString` "Stop Cheesin and jump through!")
    (else
      (set `MyPlayerClass.wallet` (+ (`MyPlayerClass.wallet` _asconnor_bp_player) 100) _asconnor_bp_player)
      (set `self.SpawnPerformed` true)
      (bind _returnvalue_2 (`|SpawnActorFromClass` "/Game/Blueprint/World/BP_RandomPlatform.BP_RandomPlatform_C" (`KismetMathLibrary.MakeTransform` (`KismetMathLibrary.MakeVector` -1200.0 0.0 (`KismetMathLibrary.Conv_IntToDouble` (* (`self.LevelCount`) 5000)))) "Undefined" "MultiplyWithRoot" null null))
      ;[1 1 1] Set Difficulty
      (set `/Game/Blueprint/World/BP_RandomPlatform.Difficulty` (- (`/Game/Blueprint/World/BP_RandomPlatform.Difficulty` _returnvalue_2) 2) _returnvalue_2)
      (`|SpawnActorFromClass` "/Game/Blueprint/World/BP_TowerBoundary.BP_TowerBoundary_C" (`KismetMathLibrary.MakeTransform` (`KismetMathLibrary.MakeVector` 0.0 0.0 (`KismetMathLibrary.Conv_IntToDouble` (* (`self.LevelCount`) 4820)))) "Undefined" "MultiplyWithRoot" null null)
      (bind _returnvalue_3 (`|SpawnActorFromClass` "BP_OneWayPlatform_C" (`KismetMathLibrary.MakeTransform` (`KismetMathLibrary.MakeVector` -1250.0 0.0 (`KismetMathLibrary.Conv_IntToDouble` (* (`self.LevelCount`) 5000)))) "Undefined" "MultiplyWithRoot" null null))
      (set `/Game/Blueprint/World/BP_OneWayPlatform.LevelCount` (+ (`self.LevelCount`) 1) _returnvalue_3)
      (bind _returnvalue_4 (`|SpawnActorFromClass` "/Game/Blueprint/World/BP_HeightBillboard.BP_HeightBillboard_C" (`KismetMathLibrary.MakeTransform` (`KismetMathLibrary.MakeVector` 2.825911 2639.087628 (`KismetMathLibrary.Conv_IntToDouble` (+ (* (`self.LevelCount`) 5000) 2530))) (struct :`Yaw` 180.0)) "Undefined" "MultiplyWithRoot" null null))
      (`TextRenderComponent.K2_SetText` (`/Game/Blueprint/World/BP_HeightBillboard.TextMiddle` _returnvalue_4) (`KismetTextLibrary.Conv_StringToText` (`KismetStringLibrary.Conv_IntToString` (+ _returnvalue 10))))
      (`TextRenderComponent.K2_SetText` (`/Game/Blueprint/World/BP_HeightBillboard.TextBottom` _returnvalue_4) (`KismetTextLibrary.Conv_StringToText` (`KismetStringLibrary.Conv_IntToString` _returnvalue)))
      (`|SpawnActorFromClass` "/Game/Blueprint/ShopAssets/BP_Shop_Door.BP_Shop_Door_C" (`KismetMathLibrary.MakeTransform` (`KismetMathLibrary.MakeVector` 900.0 0.0 (`KismetMathLibrary.Conv_IntToDouble` (* (`self.LevelCount`) 5000)))) "Undefined" "MultiplyWithRoot" null null))))

(event `InputAction|Fall through platform`
  (params (Key :type "Key Structure"))
  ;[1 1 1] Fall through platfrom (on pressing s))
)

(event `self.Above.OnComponentEndOverlap`
  (params (OverlappedComponent :type "PrimitiveComponent Object Reference") (OtherActor :type "Actor Object Reference") (OtherComp :type "PrimitiveComponent Object Reference") (OtherBodyIndex :type Integer))
  ;[1 1 1] Fall through platfrom (on pressing s))
  (cast `/Game/Blueprint/Player/BP_Player` OtherActor)
  (`self.DisableInput` (`GameplayStatics.GetPlayerController` 0))
  (`/Engine/EditorBlueprintResources/StandardMacros.Gate` true :!via `Close`
    (:`Exit`
      (`PrimitiveComponent.SetCollisionEnabled` (`self.InstancedStaticMesh`) "NoCollision"))))

(fn `UserConstructionScript`
  (for _index (range 10)
    (`InstancedStaticMeshComponent.AddInstance` (`self.InstancedStaticMesh`) (`KismetMathLibrary.MakeTransform` (`KismetMathLibrary.MakeVector` (`KismetMathLibrary.Conv_IntToDouble` (* _index 256)))) false)))