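; BP_RandomPlatform is a world actor that generates a random layout of block platforms in its construction script.
; It builds ten rows stacked along Z by accumulating PlatformSpacing, each with nine evenly spaced slots along X.
; Each slot has a one-in-four chance of adding an instanced static mesh block, up to MaxBlocks per row.
; The random X scale always resolves to 1, and the event graph is unused.
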(fn `UserConstructionScript`
  (for _ (range 10)
    (set `self.PlatformSpacing` (+ (`self.PlatformSpacing`) 2500))
    (set `self.BlockCount` 0)
    (for _index (range 9)
      (`/Engine/EditorBlueprintResources/StandardMacros.CompareInt` (`self.BlockCount`) (`self.MaxBlocks`)
        (:`<`
          (`/Engine/EditorBlueprintResources/StandardMacros.CompareInt` (`KismetMathLibrary.RandomInteger` 4) 1
            (:`<`
              (set `self.BlockCount` (+ (`self.BlockCount`) 1))
              (`InstancedStaticMeshComponent.AddInstance` (`self.InstancedStaticMesh`) (`KismetMathLibrary.MakeTransform` (`KismetMathLibrary.MakeVector` (`KismetMathLibrary.Conv_IntToDouble` (* _index 256)) 0.0 (`KismetMathLibrary.Conv_IntToDouble` (`self.PlatformSpacing`))) (struct) (`KismetMathLibrary.MakeVector` (`KismetMathLibrary.Conv_IntToDouble` (+ (`KismetMathLibrary.RandomInteger` 1) 1)) 1.0 1.0)) false))))))))