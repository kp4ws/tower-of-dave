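; AN_Landing is a Paper character animation notify that makes the player's landing kick up dust and launch nearby characters upward.
; On receipt it calls SpawnDust on BP_Player, then runs a sphere overlap for Characters around the sprite, ignoring the player.
; The sphere's offset and radius scale with the sprite's X scale, and without a valid owning instance it draws a debug sphere instead.
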(event `self.OnReceiveNotify`
  (params (OwningInstance :type "PaperZDAnimInstance Object Reference"))
  ;[1 1 1] This makes it so on land, it launches any characters in the sphere
  (`/Engine/EditorBlueprintResources/StandardMacros.IsValid` OwningInstance
    (:`Is Valid`
      (bind _asbp_player (cast `/Game/Blueprint/Player/BP_Player` (`PaperZDAnimInstance.PaperCharacter` OwningInstance)))
      (`/Game/Blueprint/Player/BP_Player.SpawnDust` _asbp_player)
      (bind _sprite (`PaperCharacter.Sprite` _asbp_player))
      (bind _relativescale3d_x (`KismetMathLibrary.BreakVector` (`SceneComponent.RelativeScale3D` _sprite)))
      (bind _outactors (`KismetSystemLibrary.SphereOverlapActors` (+ (`SceneComponent.K2_GetComponentLocation` _sprite) (* (`self.Position`) _relativescale3d_x)) (* (`self.Radius`) _relativescale3d_x) (`|MakeArray` "ObjectTypeQuery3" "ObjectTypeQuery4" :!type "EObjectTypeQuery Enum") "/Script/Engine.Character" (`|MakeArray` null _asbp_player :!type "Actor Object Reference")))
      (for _array_element _outactors
        (bind _ascharacter (cast `Character` _array_element))
        (`Character.LaunchCharacter` _ascharacter (* (`KismetMathLibrary.Vector_Up`) 1000.0) false false)))
    (:`Is Not Valid`
      (`KismetSystemLibrary.DrawDebugSphere` (`self.Position`) (`self.Radius`)))))

(fn `GetDisplayName`
  (returns (ReturnValue :type Name))
  (return (`parent.GetDisplayName`)))