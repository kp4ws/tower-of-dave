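; BP_FloorCube is a world Blueprint that builds a grid of repeated meshes from a single Instanced Static Mesh component.
; Its construction script runs three nested loops to add instances at fixed, evenly spaced local positions.
; GridSize sets both horizontal extents, while the vertical loop's end is GridSize minus a hardcoded offset, so layers appear only when GridSize reaches that offset.
; The event graph has no active logic.
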(fn `UserConstructionScript`
  (bind _gridsize (`self.GridSize`))
  (bind _returnvalue (- _gridsize 1))
  (for _index (range (+ _returnvalue 1))
    (for _index_2 (range (+ _returnvalue 1))
      (for _index_3 (range (+ (- _gridsize 250) 1))
        (`InstancedStaticMeshComponent.AddInstance` (`self.InstancedStaticMesh`) (`KismetMathLibrary.MakeTransform` (`KismetMathLibrary.MakeVector` (`KismetMathLibrary.Conv_IntToDouble` (* _index 750)) (`KismetMathLibrary.Conv_IntToDouble` (* _index_2 750)) (`KismetMathLibrary.Conv_IntToDouble` (* _index_3 750)))) false)))))