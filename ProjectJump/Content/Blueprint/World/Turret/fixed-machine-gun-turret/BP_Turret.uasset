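; Fixed turret that detects Player-tagged pawns through PawnSensing and fires a BP_Bullet after a short warning.
; On sighting, it turns its Arrow component toward the pawn and shows the Spotted indicator during a delay, which also throttles repeat sightings.
; It then plays the shot sound at the pawn's location, spawns the bullet at the Arrow's position with zero rotation, not the aim rotation, and hides the indicator.
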(event `self.PawnSensing.OnSeePawn`
  (params (Pawn :type "Pawn Object Reference"))
  (bind _returnvalue (`self.K2_GetActorLocation` Pawn))
  (if (`self.ActorHasTag` Pawn "Player")
    (`SceneComponent.K2_SetRelativeRotation` (`self.Arrow`) (`KismetMathLibrary.FindLookAtRotation` (`self.K2_GetActorLocation`) _returnvalue) false false)
    (`SceneComponent.SetVisibility` (`self.Spotted`) true false)
    (`KismetSystemLibrary.Delay` 0.8)
    (`GameplayStatics.PlaySoundAtLocation` "/Game/Blueprint/World/Turret/fixed-machine-gun-turret/pew-pew-81279_Cue.pew-pew-81279_Cue" _returnvalue (struct) 1.0 1.0 0.0 null null null null)
    (`|SpawnActorFromClass` "/Game/Blueprint/World/Turret/fixed-machine-gun-turret/BP_Bullet.BP_Bullet_C" (`KismetMathLibrary.MakeTransform` (`SceneComponent.K2_GetComponentLocation` (`self.Arrow`))) "Undefined" "MultiplyWithRoot" null null)
    (`SceneComponent.SetVisibility` (`self.Spotted`) false false)))

(fn `UserConstructionScript`)